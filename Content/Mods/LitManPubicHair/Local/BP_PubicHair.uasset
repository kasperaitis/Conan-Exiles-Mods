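; Pubic hair mod Blueprint that records a character's LowerBody mesh index as its pubic hair choice.
; On BeginPlay it saves that index to CharPubicHair for player 0 and its owning character when within 0–10, and copies a range-checked TempPubicHair to its own variable.
; ModDataTableOperations merges the race template table.
; Code that writes the value back into the character layout is disconnected, alongside debug prints.
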(event EventBeginPlay
  (CallFunction|SetTempPubicHair)
  (CallFunction|SetPubicHair)
  (CallFunction|SetCharPubicHair))

(event EventTick
  (params (DeltaSeconds :type Float%20%28single-precision%29)))

(fn ConstructionScript)

(fn ModDataTableOperations
  (Class|ModController|MergeDataTables "/Game/Systems/SpawnTable/RaceTemplateDataTable.RaceTemplateDataTable" "/Game/Mods/LitManPubicHair/RaceTemplateDataTable.RaceTemplateDataTable"))

(fn SetTempPubicHair
  (bind _asbase_player_char (Utilities|Casting|CastToBasePlayerChar (Game|GetPlayerCharacter 0)))
  (if (Math|Float|InRange(Float) (Math|Conversions|ToFloat(Integer) (.LowerBody (Utilities|Struct|BreakCharacterMeshLayout (.MeshLayout (Utilities|Struct|BreakCharacterLayout (Variables|/Game/Characters/BasePlayerChar.BasePlayerChar_C|GetCharacterLayout _asbase_player_char)))))) 0.0 1e+01)
    (Variables|/Game/Characters/BasePlayerChar.BasePlayerChar_C|SetCharPubicHair _asbase_player_char (.LowerBody (Utilities|Struct|BreakCharacterMeshLayout (.MeshLayout (Utilities|Struct|BreakCharacterLayout (Variables|/Game/Characters/BasePlayerChar.BasePlayerChar_C|GetCharacterLayout _asbase_player_char))))))))

(fn SetPubicHair
  (bind _temppubichair (Variables|Default|GetTempPubicHair))
  (Utilities|And+Branch (not (> _temppubichair 1000)) (not (< _temppubichair 0))
    (:True
      (Variables|Default|SetCharPubicHair _temppubichair))))

(fn SetCharPubicHair
  (bind _asbase_player_char (Utilities|Casting|CastToBasePlayerChar (Components|GetOwner)))
  (if (Math|Float|InRange(Float) (Math|Conversions|ToFloat(Integer) (.LowerBody (Utilities|Struct|BreakCharacterMeshLayout (.MeshLayout (Utilities|Struct|BreakCharacterLayout (Variables|/Game/Characters/BasePlayerChar.BasePlayerChar_C|GetCharacterLayout _asbase_player_char)))))) 0.0 1e+01)
    (Variables|/Game/Characters/BasePlayerChar.BasePlayerChar_C|SetCharPubicHair _asbase_player_char (.LowerBody (Utilities|Struct|BreakCharacterMeshLayout (.MeshLayout (Utilities|Struct|BreakCharacterLayout (Variables|/Game/Characters/BasePlayerChar.BasePlayerChar_C|GetCharacterLayout _asbase_player_char))))))
    (Development|PrintString (Utilities|String|Append "Character: " (Utilities|String|ToString(Integer) (.LowerBody (Utilities|Struct|BreakCharacterMeshLayout (.MeshLayout (Utilities|Struct|BreakCharacterLayout (Variables|/Game/Characters/BasePlayerChar.BasePlayerChar_C|GetCharacterLayout _asbase_player_char))))))) true true "(R=1.000000,G=0.000000,B=0.855670,A=1.000000)" 2e+01)))
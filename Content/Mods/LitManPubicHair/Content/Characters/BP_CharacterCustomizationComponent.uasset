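; Character customization component that turns a character layout into modular body-part meshes, material textures and tints, and per-slot physical materials.
; Layout changes set the master-pose mesh by gender, resolve assets, then async-load them, applying results only if they still match the latest request.
; Pausing clears the meshes and resuming rebuilds them, with server-side resolving gated by that AI LOD-seeded state.
; Mesh changes reinitialize dynamic material controllers and notify the owner.
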(event Custom|CallLayoutChanged
  (bind _returnvalue (Components|GetOwner))
  (bind _layout (Variables|Default|GetLayout))
  (bind _master (Variables|Default|GetMaster))
  (bind (_meshlayout _texturelayout _tintlayout _boolparams _intparams _scalarparams) (Utilities|Struct|BreakCharacterLayout _layout))
  (|CallParentFunction)
  (bind _returnvalue_2 (Class|CharacterLodSystem|RegisterforHighQualityHair (Class|FuncomGenericLibrary|GetCharacterLodSystem) self))
  ;[1 1 1] Not sure if this is safe, but right now it won't change much
  (Utilities|IsValid _master
    (:Is%20Valid
      (Class|SkinnedMeshComponent|SetSkeletalMesh _master (CallFunction|GetSkeletalMeshforMasterPose (.isfemale _boolparams)) false)
      (bind _shouldrun (CallFunction|ShouldRunResolve))
      (if _shouldrun
        ;[1 0 1] LitMan
        (bind (_resolvedtextures _resolvedtints _meshassetids _physicalmaterialassetids) (CallFunction|ResolveCharacterData _layout _returnvalue_2))
        (Variables|Default|SetAsyncLoadSkeletalMeshAssets _meshassetids)
        (Variables|Default|SetAsyncLoadPhysicalMaterials _physicalmaterialassetids)
        (Class|CharacterCustomizationComponent|SetMaterialParams (Utilities|Struct|MakeCharacterMaterialParams _resolvedtextures _resolvedtints _scalarparams) false)
        (Class|CharacterCustomizationComponent|ArmourDyeUpdated)
        ;[1 0.9867 0.9186] We should definitely move this to code. For noew I made this abstract art to prevent cases where Asset A starts async load, then B starts, but B is already loaded so A finishes loading after B and ends up overwriting the mesh. This fixed some cases of female characters spawning as male.
        (bind _loadedobjects (|LoadAssetsAsync _meshassetids)
          (:then
            (bind _loadedobjects_2 (|LoadAssetsAsync _physicalmaterialassetids)
              (:OnLoaded
                (bind _enumvalue (|ForEachCharacterBodySlots)
                  (:LoopBody
                    (if (== (Utilities|ResolveSoftReference (Utilities|Array|Get(acopy) (Variables|Default|GetAsyncLoadPhysicalMaterials) (Math|Conversions|ToInteger(Byte) _enumvalue))) (Utilities|Array|Get(acopy) _loadedobjects_2 (Math|Conversions|ToInteger(Byte) _enumvalue)))
                      (CallFunction|UpdateHitLocationPhysicalMaterial (Components|GetOwner) _enumvalue (.AsPhysical%20Material (Utilities|Casting|CastToPhysicalMaterial (Utilities|Array|Get(acopy) _loadedobjects_2 (Math|Conversions|ToInteger(Byte) _enumvalue)))))))
                  (:then
                    (if (Utilities|DoesObjectImplementInterface _returnvalue "/Game/Characters/CharacterCustomizationInterface.CharacterCustomizationInterface_C")
                      (Class|CharacterCustomizationInterface|OnPhysicsMaterialChanged(Message) _returnvalue)))))))
          (:OnLoaded
            (if (Math|Boolean|ANDBoolean (== (Utilities|Array|Get(acopy) _loadedobjects) (Utilities|ResolveSoftReference (Utilities|Array|Get(acopy) (Variables|Default|GetAsyncLoadSkeletalMeshAssets)))) (== (Utilities|Array|Get(acopy) _loadedobjects 1) (Utilities|ResolveSoftReference (Utilities|Array|Get(acopy) (Variables|Default|GetAsyncLoadSkeletalMeshAssets) 1))) (== (Utilities|Array|Get(acopy) _loadedobjects 2) (Utilities|ResolveSoftReference (Utilities|Array|Get(acopy) (Variables|Default|GetAsyncLoadSkeletalMeshAssets) 2))) (== (Utilities|Array|Get(acopy) _loadedobjects 3) (Utilities|ResolveSoftReference (Utilities|Array|Get(acopy) (Variables|Default|GetAsyncLoadSkeletalMeshAssets) 3))) (== (Utilities|Array|Get(acopy) _loadedobjects 4) (Utilities|ResolveSoftReference (Utilities|Array|Get(acopy) (Variables|Default|GetAsyncLoadSkeletalMeshAssets) 4))) (== (Utilities|Array|Get(acopy) _loadedobjects 5) (Utilities|ResolveSoftReference (Utilities|Array|Get(acopy) (Variables|Default|GetAsyncLoadSkeletalMeshAssets) 5))) (== (Utilities|Array|Get(acopy) _loadedobjects 6) (Utilities|ResolveSoftReference (Utilities|Array|Get(acopy) (Variables|Default|GetAsyncLoadSkeletalMeshAssets) 6))) (== (Utilities|Array|Get(acopy) _loadedobjects 7) (Utilities|ResolveSoftReference (Utilities|Array|Get(acopy) (Variables|Default|GetAsyncLoadSkeletalMeshAssets) 7))) (== (Utilities|Array|Get(acopy) _loadedobjects 8) (Utilities|ResolveSoftReference (Utilities|Array|Get(acopy) (Variables|Default|GetAsyncLoadSkeletalMeshAssets) 8))) (== (Utilities|Array|Get(acopy) _loadedobjects 9) (Utilities|ResolveSoftReference (Utilities|Array|Get(acopy) (Variables|Default|GetAsyncLoadSkeletalMeshAssets) 9))))
              (Class|CharacterCustomizationComponent|SetMeshes (Utilities|Struct|MakeCharacterResolvedMeshes (Utilities|ResolveSoftReference (Utilities|Array|Get(acopy) (Variables|Default|GetAsyncLoadSkeletalMeshAssets))) (Utilities|ResolveSoftReference (Utilities|Array|Get(acopy) (Variables|Default|GetAsyncLoadSkeletalMeshAssets) 1)) (Utilities|ResolveSoftReference (Utilities|Array|Get(acopy) (Variables|Default|GetAsyncLoadSkeletalMeshAssets) 9)) (Utilities|ResolveSoftReference (Utilities|Array|Get(acopy) (Variables|Default|GetAsyncLoadSkeletalMeshAssets) 2)) (Utilities|ResolveSoftReference (Utilities|Array|Get(acopy) (Variables|Default|GetAsyncLoadSkeletalMeshAssets) 3)) (Utilities|ResolveSoftReference (Utilities|Array|Get(acopy) (Variables|Default|GetAsyncLoadSkeletalMeshAssets) 4)) (Utilities|ResolveSoftReference (Utilities|Array|Get(acopy) (Variables|Default|GetAsyncLoadSkeletalMeshAssets) 5)) (Utilities|ResolveSoftReference (Utilities|Array|Get(acopy) (Variables|Default|GetAsyncLoadSkeletalMeshAssets) 6)) (Utilities|ResolveSoftReference (Utilities|Array|Get(acopy) (Variables|Default|GetAsyncLoadSkeletalMeshAssets) 7)) (Utilities|ResolveSoftReference (Utilities|Array|Get(acopy) (Variables|Default|GetAsyncLoadSkeletalMeshAssets) 8))) false)
              (Class|CharacterLodSystem|UpdateClothSimAdjustmentRegistration (Class|FuncomGenericLibrary|GetCharacterLodSystem) (Components|GetOwner))
              (Default|CallOnSkeletalMeshInitialized))))))))

(event EventBeginPlay)

(event EventTick
  (params (DeltaSeconds :type Float%20%28single-precision%29))
  (|CallParentFunction DeltaSeconds))

(event EventOnMeshesChanged
  (|CallParentFunction)
  (CallFunction|OnMeshesChangedInternal))

(event EventOnPause
  (Variables|Default|SetIsResumed false)
  (if (Variables|Default|GetEnabled)
    (Class|CharacterCustomizationComponent|SetMeshes (Utilities|Struct|MakeCharacterResolvedMeshes 0 0 0 0 0 0 0 0 0 0) false)))

(event EventOnLayoutChanged
  (bind _returnvalue (Components|GetOwner))
  (bind _layout (Variables|Default|GetLayout))
  (bind _master (Variables|Default|GetMaster))
  (bind (_meshlayout _texturelayout _tintlayout _boolparams _intparams _scalarparams) (Utilities|Struct|BreakCharacterLayout _layout))
  (|CallParentFunction)
  (bind _returnvalue_2 (Class|CharacterLodSystem|RegisterforHighQualityHair (Class|FuncomGenericLibrary|GetCharacterLodSystem) self))
  ;[1 1 1] Not sure if this is safe, but right now it won't change much
  (Utilities|IsValid _master
    (:Is%20Valid
      (Class|SkinnedMeshComponent|SetSkeletalMesh _master (CallFunction|GetSkeletalMeshforMasterPose (.isfemale _boolparams)) false)
      (bind _shouldrun (CallFunction|ShouldRunResolve))
      (if _shouldrun
        ;[1 0 1] LitMan
        (bind (_resolvedtextures _resolvedtints _meshassetids _physicalmaterialassetids) (CallFunction|ResolveCharacterData _layout _returnvalue_2))
        (Variables|Default|SetAsyncLoadSkeletalMeshAssets _meshassetids)
        (Variables|Default|SetAsyncLoadPhysicalMaterials _physicalmaterialassetids)
        (Class|CharacterCustomizationComponent|SetMaterialParams (Utilities|Struct|MakeCharacterMaterialParams _resolvedtextures _resolvedtints _scalarparams) false)
        (Class|CharacterCustomizationComponent|ArmourDyeUpdated)
        ;[1 0.9867 0.9186] We should definitely move this to code. For noew I made this abstract art to prevent cases where Asset A starts async load, then B starts, but B is already loaded so A finishes loading after B and ends up overwriting the mesh. This fixed some cases of female characters spawning as male.
        (bind _loadedobjects (|LoadAssetsAsync _meshassetids)
          (:then
            (bind _loadedobjects_2 (|LoadAssetsAsync _physicalmaterialassetids)
              (:OnLoaded
                (bind _enumvalue (|ForEachCharacterBodySlots)
                  (:LoopBody
                    (if (== (Utilities|ResolveSoftReference (Utilities|Array|Get(acopy) (Variables|Default|GetAsyncLoadPhysicalMaterials) (Math|Conversions|ToInteger(Byte) _enumvalue))) (Utilities|Array|Get(acopy) _loadedobjects_2 (Math|Conversions|ToInteger(Byte) _enumvalue)))
                      (CallFunction|UpdateHitLocationPhysicalMaterial (Components|GetOwner) _enumvalue (.AsPhysical%20Material (Utilities|Casting|CastToPhysicalMaterial (Utilities|Array|Get(acopy) _loadedobjects_2 (Math|Conversions|ToInteger(Byte) _enumvalue)))))))
                  (:then
                    (if (Utilities|DoesObjectImplementInterface _returnvalue "/Game/Characters/CharacterCustomizationInterface.CharacterCustomizationInterface_C")
                      (Class|CharacterCustomizationInterface|OnPhysicsMaterialChanged(Message) _returnvalue)))))))
          (:OnLoaded
            (if (Math|Boolean|ANDBoolean (== (Utilities|Array|Get(acopy) _loadedobjects) (Utilities|ResolveSoftReference (Utilities|Array|Get(acopy) (Variables|Default|GetAsyncLoadSkeletalMeshAssets)))) (== (Utilities|Array|Get(acopy) _loadedobjects 1) (Utilities|ResolveSoftReference (Utilities|Array|Get(acopy) (Variables|Default|GetAsyncLoadSkeletalMeshAssets) 1))) (== (Utilities|Array|Get(acopy) _loadedobjects 2) (Utilities|ResolveSoftReference (Utilities|Array|Get(acopy) (Variables|Default|GetAsyncLoadSkeletalMeshAssets) 2))) (== (Utilities|Array|Get(acopy) _loadedobjects 3) (Utilities|ResolveSoftReference (Utilities|Array|Get(acopy) (Variables|Default|GetAsyncLoadSkeletalMeshAssets) 3))) (== (Utilities|Array|Get(acopy) _loadedobjects 4) (Utilities|ResolveSoftReference (Utilities|Array|Get(acopy) (Variables|Default|GetAsyncLoadSkeletalMeshAssets) 4))) (== (Utilities|Array|Get(acopy) _loadedobjects 5) (Utilities|ResolveSoftReference (Utilities|Array|Get(acopy) (Variables|Default|GetAsyncLoadSkeletalMeshAssets) 5))) (== (Utilities|Array|Get(acopy) _loadedobjects 6) (Utilities|ResolveSoftReference (Utilities|Array|Get(acopy) (Variables|Default|GetAsyncLoadSkeletalMeshAssets) 6))) (== (Utilities|Array|Get(acopy) _loadedobjects 7) (Utilities|ResolveSoftReference (Utilities|Array|Get(acopy) (Variables|Default|GetAsyncLoadSkeletalMeshAssets) 7))) (== (Utilities|Array|Get(acopy) _loadedobjects 8) (Utilities|ResolveSoftReference (Utilities|Array|Get(acopy) (Variables|Default|GetAsyncLoadSkeletalMeshAssets) 8))) (== (Utilities|Array|Get(acopy) _loadedobjects 9) (Utilities|ResolveSoftReference (Utilities|Array|Get(acopy) (Variables|Default|GetAsyncLoadSkeletalMeshAssets) 9))))
              (Class|CharacterCustomizationComponent|SetMeshes (Utilities|Struct|MakeCharacterResolvedMeshes (Utilities|ResolveSoftReference (Utilities|Array|Get(acopy) (Variables|Default|GetAsyncLoadSkeletalMeshAssets))) (Utilities|ResolveSoftReference (Utilities|Array|Get(acopy) (Variables|Default|GetAsyncLoadSkeletalMeshAssets) 1)) (Utilities|ResolveSoftReference (Utilities|Array|Get(acopy) (Variables|Default|GetAsyncLoadSkeletalMeshAssets) 9)) (Utilities|ResolveSoftReference (Utilities|Array|Get(acopy) (Variables|Default|GetAsyncLoadSkeletalMeshAssets) 2)) (Utilities|ResolveSoftReference (Utilities|Array|Get(acopy) (Variables|Default|GetAsyncLoadSkeletalMeshAssets) 3)) (Utilities|ResolveSoftReference (Utilities|Array|Get(acopy) (Variables|Default|GetAsyncLoadSkeletalMeshAssets) 4)) (Utilities|ResolveSoftReference (Utilities|Array|Get(acopy) (Variables|Default|GetAsyncLoadSkeletalMeshAssets) 5)) (Utilities|ResolveSoftReference (Utilities|Array|Get(acopy) (Variables|Default|GetAsyncLoadSkeletalMeshAssets) 6)) (Utilities|ResolveSoftReference (Utilities|Array|Get(acopy) (Variables|Default|GetAsyncLoadSkeletalMeshAssets) 7)) (Utilities|ResolveSoftReference (Utilities|Array|Get(acopy) (Variables|Default|GetAsyncLoadSkeletalMeshAssets) 8))) false)
              (Class|CharacterLodSystem|UpdateClothSimAdjustmentRegistration (Class|FuncomGenericLibrary|GetCharacterLodSystem) (Components|GetOwner))
              (Default|CallOnSkeletalMeshInitialized))))))))

(event EventOnResume
  (Variables|Default|SetIsResumed true)
  (if (Variables|Default|GetEnabled)
    (CallFunction|CallLayoutChanged)))

(fn OnMeshesChangedInternal
  (bind _output_get (LocalVariables|SetOwner_ (Components|GetOwner)))
  (bind _output_get_2 (LocalVariables|SetDynamicMaterialParameterControllers_ (Actor|GetComponentsByClass _output_get "/Game/Effects/blueprints/DynamicMaterialParamController.DynamicMaterialParamController_C")))
  (for _array_element _output_get_2
    (Default|Initialize _array_element))
  (if (Utilities|DoesObjectImplementInterface _output_get "/Game/Characters/CharacterCustomizationInterface.CharacterCustomizationInterface_C")
    (Class|CharacterCustomizationInterface|OnMeshesChanged(Message) _output_get)))

(fn ResolveCharacterDataInternal
  (params (InLayout :type Character%20Layout%20Structure%20%28by%20ref%29) (AllowHighQualityHair :type Boolean))
  ;[1 0 1] LitMan
  (bind (_resolvedtextures _resolvedtints _meshassetids _physicalmaterialassetids) (CallFunction|ResolveCharacterData InLayout AllowHighQualityHair))
  (return _resolvedtextures _resolvedtints _meshassetids _physicalmaterialassetids))

(fn ShouldRunResolve
  (bind _returnvalue (Components|GetOwner))
  (bind _returnvalue_2 (Actor|GetComponentbyClass _returnvalue "/Script/ConanSandbox.AILODComponent"))
  (if (Networking|IsServer)
    (if (Utilities|IsValid (Variables|Default|GetCachedLodComponent))
      (return (Variables|Default|GetIsResumed))
      (else
        (Utilities|IsValid _returnvalue_2
          (:Is%20Valid
            (bind _output_get (Variables|Default|SetCachedLodComponent _returnvalue_2))
            (Variables|Default|SetIsResumed (< (Variables|/Script/ConanSandbox.AILODComponent|GetAILOD _output_get) 3))
            (return (Variables|Default|GetIsResumed)))
          (:Is%20Not%20Valid
            _)))))
  (return true))

(fn GetCustomTickInterval
  (params (newLOD :type Integer))
  (return 0.0))

(fn HasCustomTickInterval
  (return false))

(fn TickIndependentPauseResume
  (return true))
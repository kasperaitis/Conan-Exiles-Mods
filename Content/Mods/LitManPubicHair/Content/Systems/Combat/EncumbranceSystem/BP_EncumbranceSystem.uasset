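; Encumbrance component that tracks a Conan character's carried weight and derives its encumbrance tier.
; Inventory signals drive incremental server-side updates to the weight stat, which is measured against a maximum from base, progression bonus and perk.
; The tier selects a stamina effect; lower tiers restore original crouch and swim speeds.
; The top tier shows a throttled warning, or kills characters carrying people past a limit, awarding those carried an achievement.
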(event Custom|SlotCurrentEncumbranceChanged
  (params (actor :type Actor%20Object%20Reference) (statID :type ECharFloatStatID%20Enum) (newValue :type Float%20%28single-precision%29) (deltaValue :type Float%20%28single-precision%29))
  (Default|CallSignalEncumbranceChanged)
  (CallFunction|HandleCharacterEncumbrance))

(event EventOnRepCurrentEncumbranceTier
  (bind _comp (CallFunction|GetCharacterMovementComp))
  (if (Utilities|Enum|NotEqual(Enum) (Variables|Default|GetCurrentEncumbranceTier) "Tier4")
    (Variables|/Script/Engine.CharacterMovementComponent|SetMaxWalkSpeedCrouched _comp (Variables|Default|GetOriginalMaxCrouchedWalkSpeed))
    (Variables|/Script/Engine.CharacterMovementComponent|SetMaxSwimSpeed _comp (Variables|Default|GetOriginalMaxSwimSpeed))))

(event EventDataLoaded
  (|CallParentFunction)
  (Variables|Default|SetHas%20Initialized true)
  (bind _asconan_character (Utilities|Casting|CastToConanCharacter (Components|GetOwner)))
  (Class|ConanCharacter|SetFloatStat _asconan_character "CurrentEncumbrance" 0.0)
  (bind _returnvalue (Class|ConanCharacter|GetFloatStatChangeSignal _asconan_character "CurrentEncumbrance"))
  (EventDispatchers|BindEventtoSignalStatChanged _returnvalue (delegate Custom|SlotCurrentEncumbranceChanged))
  (bind _ascharacter_movement_component (Utilities|Casting|CastToCharacterMovementComponent (Pawn|GetMovementComponent _asconan_character)))
  (Variables|Default|SetOriginalMaxSwimSpeed (Variables|/Script/Engine.CharacterMovementComponent|GetMaxSwimSpeed _ascharacter_movement_component))
  (Variables|Default|SetOriginalMaxCrouchedWalkSpeed (Variables|/Script/Engine.CharacterMovementComponent|GetMaxWalkSpeedCrouched _ascharacter_movement_component))
  (|SetCharacterMovement
    (:exit
      (|SetProgressionSystem
        (:else
          (|SetBackpackInventory)
          (|SetEquipmentInventory)
          (|SetHotbarInventory)
          (|ProcessInventories
            (:Completed
              (|BindInventorySignals))))))))

(fn HandleCharacterEncumbrance
  (if (Networking|IsServer)
    (if (Variables|Default|GetHas%20Initialized)
      (bind _asconan_character (Utilities|Casting|CastToConanCharacter (Components|GetOwner)))
      (LocalVariables|SetCurrentEncumbranceLevel (/ (Class|ConanCharacter|GetFloatStat _asconan_character "CurrentEncumbrance" "Full") (CallFunction|GetEncumbranceMax)))
      (Variables|Default|SetCurrentEncumbranceTier "Tier4")
      (bind (_array_element _array_index) (Utilities|Array|ForEachLoopwithBreak (Variables|Default|GetEncumbranceTierThresholds) :!label _label)
        (:LoopBody
          (if (>= _array_element (LocalVariables|GetCurrentEncumbranceLevel))
            (Variables|Default|SetCurrentEncumbranceTier (Utilities|Enum|ByteToEnumEEncumbranceTiers (Math|Conversions|ToByte(Integer) _array_index)))
            (goto _label Break)))
        (:Completed
          (CallFunction|HandleOverWeight))))))

(fn GetEncumbranceStaminaEffect
  ;[1 1 1] Check for cheats like a c++ maestro =3
  (bind _asconan_character (Utilities|Casting|CastToConanCharacter (Components|GetOwner))
    (:then
      (if (Variables|/Script/ConanSandbox.ConanCharacter|GetSprintNoCost _asconan_character)
        (return 0.0)
        (else
          _)))
    (:CastFailed
      _))
  (return (Utilities|Array|Get(acopy) (Variables|Default|GetEncumbranceStaminaEffect) (Math|Conversions|ToInteger(Byte) (Variables|Default|GetCurrentEncumbranceTier)))))

(fn HandleOverWeight
  (bind _comp (CallFunction|GetCharacterMovementComp))
  (if (Utilities|Enum|Equal(Enum) (Variables|Default|GetCurrentEncumbranceTier) "Tier4")
    (bind _asconan_character (Utilities|Casting|CastToConanCharacter (Components|GetOwner)))
    (if (and (> (Utilities|Array|Length (Variables|/Script/ConanSandbox.ConanCharacter|GetCarriedPeople _asconan_character)) 0) (>= (/ (Class|ConanCharacter|GetFloatStat _asconan_character "CurrentEncumbrance" "Full") (CallFunction|GetEncumbranceMax)) (Variables|Default|GetCarryPeopleLimit)))
      (bind _asis_base_bpcombat_interface (Utilities|Casting|CastToIsBaseBPCombatInterface _asconan_character)
        (:then
          ;[1 1 1] Give achievement to all players on top of the dying character
          (for _array_element (Variables|/Script/ConanSandbox.ConanCharacter|GetCarriedPeople _asconan_character)
            (if (> (Utilities|Array|Length (Actor|GetComponentsbyTag (Pawn|GetController _array_element) "/Script/Engine.ActorComponent" "AchievementSystem")) 0)
              (bind _asachievement_interface (Utilities|Casting|CastToAchievementInterface (Utilities|Array|Get(acopy) (Actor|GetComponentsbyTag (Pawn|GetController _array_element) "/Script/Engine.ActorComponent" "AchievementSystem"))))
              (Default|GiveAchievementProgressInterfaceFunc _asachievement_interface "ACH_PeerPressure" 1e+02)))
          (Default|KillCharacterInterface _asis_base_bpcombat_interface "RightLegLower" "too much pressure" "NewEnumerator9"))
        (:CastFailed
          (if (< (+ (Variables|Default|GetTimeFIDOSinceLast) (Variables|Default|GetTimeFIFOCooldown)) (Utilities|Time|GetGameTimeinSeconds)) :!label _label
            (Class|ConanCharacter|ClientHUDShowFIFOatLocation _asconan_character (Utilities|Text|FormatText "You are over encumbered") "Low")
            (Variables|Default|SetTimeFIDOSinceLast (Utilities|Time|GetGameTimeinSeconds)))))
      (else
        (goto _label)))
    (else
      (Variables|/Script/Engine.CharacterMovementComponent|SetMaxWalkSpeedCrouched _comp (Variables|Default|GetOriginalMaxCrouchedWalkSpeed))
      (Variables|/Script/Engine.CharacterMovementComponent|SetMaxSwimSpeed _comp (Variables|Default|GetOriginalMaxSwimSpeed)))))

(fn HandleItemEncumbrance
  (params (GameItem :type Game%20Item%20Object%20Reference) (NewItem :type Boolean) (StackChangeDelta :type Integer))
  (Utilities|IsValid GameItem
    (:Is%20Valid
      (if (Networking|IsServer)
        (Utilities|FlowControl|Sequence
          (:then_0
            (LocalVariables|Setlocal%20GameItem GameItem))
          (:then_1
            (LocalVariables|Setlocal%20NewItem NewItem))
          (:then_2
            (LocalVariables|Setlocal%20StackChangeDelta StackChangeDelta))
          (:then_3
            (if (not (Class|GameItem|IsShortcut (LocalVariables|Getlocal%20GameItem)))
              (if (!= (LocalVariables|Getlocal%20StackChangeDelta) 0)
                ;[1 1 1] Handle Stack size change
                (LocalVariables|Setlocal%20WeightDelta (* (LocalVariables|Getlocal%20StackChangeDelta) (Class|GameItem|GetFloatStat (LocalVariables|Getlocal%20GameItem) "EncumbranceWeight")))
                (else
                  ;[1 1 1] Handle adding or removing whole items, including item with a stack
                  (LocalVariables|Setlocal%20WeightDelta (* (* (Math|Integer|SelectInt (Class|GameItem|GetIntStat (LocalVariables|Getlocal%20GameItem) "StackSize") 1 (> (Class|GameItem|GetIntStat (LocalVariables|Getlocal%20GameItem) "MaxStackSize") 0)) (Class|GameItem|GetFloatStat (LocalVariables|Getlocal%20GameItem) "EncumbranceWeight")) (Math|Float|SelectFloat 1.0 -1.0 (LocalVariables|Getlocal%20NewItem))))))
              (bind _asconan_character (Utilities|Casting|CastToConanCharacter (Components|GetOwner)))
              (Class|ConanCharacter|SetFloatStat _asconan_character "CurrentEncumbrance" (+ (Class|ConanCharacter|GetFloatStat _asconan_character "CurrentEncumbrance" "Base") (LocalVariables|Getlocal%20WeightDelta)))
              (CallFunction|HandleCharacterEncumbrance)))
          (:then_4
            (bind _asconan_character_2 (Utilities|Casting|CastToConanCharacter (Components|GetOwner)))
            (Class|ConanCharacter|RecalculateCarriedPeopleWeight _asconan_character_2)))))))

(fn GetEncumbranceMax
  (bind _returnvalue (Components|GetOwner))
  (bind _progressionsystem (Variables|Default|GetProgressionSystem))
  (bind _returnvalue_2 (Actor|GetComponentbyClass _returnvalue "/Game/Systems/Perks/BP_PerkSystemComponent.BP_PerkSystemComponent_C"))
  (Utilities|IsValid _progressionsystem
    (:Is%20Valid
      (if (Utilities|DoesObjectImplementInterface (Components|GetOwner) "/Game/Systems/Interfaces/BasePlayerCharInterface.BasePlayerCharInterface_C")
        (bind _hasperk (Default|HasPerk _returnvalue_2 "Encumberance_30"))
        (if _hasperk
          (bind _modifier (Default|GetPerksEncumberanceModifier _returnvalue_2))
          (return (* _modifier (+ (Variables|Default|GetEncumbranceBase) (Variables|/Game/Systems/Progression/BP_ProgressionSystem.BP_ProgressionSystem_C|GetBonusEncumbrance (Variables|Default|GetProgressionSystem)))))
          (else
            _)))
      (return (+ (Variables|Default|GetEncumbranceBase) (Variables|/Game/Systems/Progression/BP_ProgressionSystem.BP_ProgressionSystem_C|GetBonusEncumbrance _progressionsystem))))
    (:Is%20Not%20Valid
      (return (Variables|Default|GetEncumbranceBase)))))

(fn OnRepEncumbranceCurrent
  (Default|CallSignalEncumbranceChanged))

(fn OnRepEncumbranceBase
  (Default|CallSignalEncumbranceChanged))

(fn GetCharacterMovementComp
  (bind _returnvalue (Components|GetOwner))
  (bind _returnvalue_2 (Actor|GetComponentsByClass _returnvalue "/Script/Engine.CharacterMovementComponent"))
  (bind _charactermovement (Variables|Default|GetCharacterMovement)
    (:then
      (return _charactermovement))
    (:else
      (if (> (Utilities|Array|Length _returnvalue_2) 0)
        (bind _output_get (Variables|Default|SetCharacterMovement (Utilities|Array|Get(acopy) _returnvalue_2)))
        (return _output_get)
        (else
          (return 0))))))

(event Custom|SignalItemFloatStatChanged_Encumbrance
  (params (item :type Game%20Item%20Object%20Reference) (statID :type EItemFloatStatID%20Enum) (statValue :type Float%20%28single-precision%29) (deltaValue :type Float%20%28single-precision%29))
  ;[1 1 1] Bind all inventories to Add Item and remove Item signals
  (if (Utilities|Enum|Equal(Enum) statID "EncumbranceWeight")
    (bind _asconan_character (Utilities|Casting|CastToConanCharacter (Components|GetOwner)))
    (Class|ConanCharacter|SetFloatStat _asconan_character "CurrentEncumbrance" (+ (Class|ConanCharacter|GetFloatStat _asconan_character "CurrentEncumbrance" "Base") deltaValue))
    (CallFunction|HandleCharacterEncumbrance)))

(event Custom|SignalItemIntStatChanged_Encumbrance
  (params (item :type Game%20Item%20Object%20Reference) (statID :type EItemIntStatID%20Enum) (statValue :type Integer) (deltaValue :type Integer))
  ;[1 1 1] Bind all inventories to Add Item and remove Item signals
  (if (Utilities|Enum|Equal(Enum) statID "StackSize")
    (CallFunction|HandleItemEncumbrance item false deltaValue)))

(event Custom|SignalItemAdded_Encumbrance
  (params (index :type Integer) (item :type Game%20Item%20Object%20Reference) (srcInventory :type Item%20Inventory%20Object%20Reference) (srcIndex :type Integer))
  ;[1 1 1] Bind all inventories to Add Item and remove Item signals
  (CallFunction|HandleItemEncumbrance item true))

(event Custom|SignalItemRemoved_Encumbrance
  (params (index :type Integer) (item :type Game%20Item%20Object%20Reference) (dstInventory :type Item%20Inventory%20Object%20Reference) (dstIndex :type Integer))
  ;[1 1 1] Bind all inventories to Add Item and remove Item signals
  (CallFunction|HandleItemEncumbrance item false))

(fn GetEncumbranceTier
  (return (Variables|Default|GetCurrentEncumbranceTier)))
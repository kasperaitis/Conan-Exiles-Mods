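; Actor component that drives a named scalar material parameter on its owner's meshes and fades it back toward a default value over time.
; Initialize, skipped on dedicated servers, creates dynamic material instances for primitive component materials that have the parameter.
; Set and Add functions clamp the value between target and default, enabling tick only while below default with positive fade rate.
; The "Blood amount" parameter changes only when blood is allowed.
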(event EventBeginPlay)

(event EventTick
  (params (DeltaSeconds :type Float%20%28single-precision%29))
  (CallFunction|AddtoParamValue (* DeltaSeconds (Variables|Default|GetFadeDirection) (Variables|Default|GetFadeRate))))

(fn Initialize
  (Utilities|Array|Clear (Variables|Default|GetDynamicMaterialInstances))
  (if (not (Networking|IsDedicatedServer))
    (bind _output_get (LocalVariables|SetPrimitiveComponents_ (Actor|GetComponentsByClass (Components|GetOwner) "/Script/Engine.PrimitiveComponent")))
    (for _array_element _output_get
      (for _index (range 0 (- (Rendering|Material|GetNumMaterials _array_element) 1))
        (bind _output_get_2 (LocalVariables|SetCurrentMaterialInterface (Rendering|Material|GetMaterial _array_element _index)))
        (bind _returnvalue (Class|EnvironmentFunctionLibrary|DoesMaterialHaveScalarParameter _output_get_2 (Variables|Default|GetParamName)))
        (if _returnvalue
          (bind _returnvalue_2 (Rendering|Material|CreateDynamicMaterialInstance _array_element _index _output_get_2 :!class /Script/Engine.PrimitiveComponent))
          (Utilities|Array|Add (Variables|Default|GetDynamicMaterialInstances) _returnvalue_2))))
    (CallFunction|SetParamValue (Variables|Default|GetDefaultVal))
    (Variables|Default|SetFadeDirection (Math|Float|Sign(Float) (- (Variables|Default|GetDefaultVal) (Variables|Default|GetTargetVal))))))

(fn AddtoParamValue
  (params (Amount :type Float%20%28single-precision%29))
  (bind _dynamicmaterialinstances (Variables|Default|GetDynamicMaterialInstances))
  (bind _targetval (Variables|Default|GetTargetVal))
  (bind _defaultval (Variables|Default|GetDefaultVal))
  (if (> (Utilities|Array|Length _dynamicmaterialinstances) 0)
    (if (or (Class|CensoredContentHelper|IsBloodAllowed) (Utilities|Name|NotEqual(Name) (Variables|Default|GetParamName) "Blood amount"))
      (bind _output_get (Variables|Default|SetParamVal (Math|Float|Clamp(Float) (+ Amount (Variables|Default|GetParamVal)) (Math|Float|Min(Float) _targetval _defaultval) (Math|Float|Max(Float) _targetval _defaultval))))
      (LocalVariables|SetEnabled_ (and (< _output_get (Variables|Default|GetDefaultVal)) (> (Variables|Default|GetFadeRate) 0.0)))
      (for _array_element _dynamicmaterialinstances
        (Rendering|Material|SetScalarParameterValue _array_element (Variables|Default|GetParamName) _output_get :!class /Script/Engine.MaterialInstanceDynamic)
        (Components|Tick|SetComponentTickEnabled (LocalVariables|GetEnabled_))))))

(fn SetParamValue
  (params (Value :type Float%20%28single-precision%29))
  (bind _dynamicmaterialinstances (Variables|Default|GetDynamicMaterialInstances))
  (bind _targetval (Variables|Default|GetTargetVal))
  (bind _defaultval (Variables|Default|GetDefaultVal))
  (if (> (Utilities|Array|Length _dynamicmaterialinstances) 0)
    (if (or (Class|CensoredContentHelper|IsBloodAllowed) (Utilities|Name|NotEqual(Name) (Variables|Default|GetParamName) "Blood amount"))
      (bind _output_get (Variables|Default|SetParamVal (Math|Float|Clamp(Float) Value (Math|Float|Min(Float) _targetval _defaultval) (Math|Float|Max(Float) _targetval _defaultval))))
      (bind _output_get_2 (LocalVariables|SetEnabled (and (< _output_get (Variables|Default|GetDefaultVal)) (> (Variables|Default|GetFadeRate) 0.0))))
      (for _array_element _dynamicmaterialinstances
        (Rendering|Material|SetScalarParameterValue _array_element (Variables|Default|GetParamName) _output_get :!class /Script/Engine.MaterialInstanceDynamic)
        (Components|Tick|SetComponentTickEnabled _output_get_2))
      (else
        (Components|Tick|SetComponentTickEnabled false :!label _label)))
    (else
      (goto _label))))
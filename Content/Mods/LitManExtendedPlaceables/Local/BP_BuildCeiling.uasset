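; BP_BuildCeiling is a buildable ceiling piece in the LitManExtendedPlaceables mod that cannot be placed where stairs block it.
; Its CanBePlaced override runs the parent check first, then, if that result ranks below Fail, sweeps StairCheckerBox downwards for BP_BuildStairs.
; A detected stair returns Fail with a blocked-by-stair message; otherwise the parent result passes through.
; The event graph and construction script add no logic.
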(event EventBeginPlay
  (|CallParentFunction))

(event Collision|EventActorBeginOverlap
  (params (OtherActor :type Actor%20Object%20Reference))
  (|CallParentFunction 0))

(event EventTick
  (params (DeltaSeconds :type Float%20%28single-precision%29)))

(fn ConstructionScript
  (|CallParentFunction))

(fn CanbePlaced
  (params (AttachTo :type Buildable%20Base%20Object%20Reference) (InstanceIndex :type Integer))
  (bind (_failedmessage _returnvalue) (|CallParentFunction AttachTo InstanceIndex))
  (if (< (Math|Conversions|ToInteger(Byte) _returnvalue) (Math|Conversions|ToInteger(Byte) (Utilities|Enum|LiteralenumECanBePlacedResult "Fail")))
    (bind _foundoverlaps (CallFunction|CheckforOverlappingStructure (Variables|Default|GetStairCheckerBox) 16.0 (Utilities|Array|MakeArray "/Game/Systems/Building/BP_BuildStairs.BP_BuildStairs_C")))
    (if _foundoverlaps
      (return (Utilities|String|ToString(Text) (Variables|Default|GetError_BlockedByStair)) "Fail")
      (else
        (return _failedmessage _returnvalue)))
    (else
      (return _failedmessage _returnvalue))))
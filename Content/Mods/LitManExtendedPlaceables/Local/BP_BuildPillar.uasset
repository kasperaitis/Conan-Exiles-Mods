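; Buildable pillar placeable from the LitManExtendedPlaceables mod, with custom placement validation.
; CanBePlaced returns the parent result if socket-snapped; otherwise a short vertical WorldStatic multi-trace must find static ground, or placement fails with a landscape-or-socket error.
; An unreachable EventGraph block holds a disabled attempt to auto-fill instanced pillar meshes and build sockets down to the ground.
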(event EventBeginPlay
  (|CallParentFunction))

(event Collision|EventActorBeginOverlap
  (params (OtherActor :type Actor%20Object%20Reference))
  (|CallParentFunction 0))

(event EventTick
  (params (DeltaSeconds :type Float%20%28single-precision%29))
  (|CallParentFunction 0.0))

(fn ConstructionScript
  (|CallParentFunction))

(fn CanbePlaced
  (params (AttachTo :type Buildable%20Base%20Object%20Reference) (InstanceIndex :type Integer))
  (bind _returnvalue (Transformation|GetActorLocation))
  (bind (_failedmessage _returnvalue_2) (|CallParentFunction AttachTo InstanceIndex))
  ;[1 1 1] Check if overlapping with landscape
  (if (Variables|Default|GetIsSnappedToSocket)
    _
    (else
      (bind _outhits (Class|KismetSystemLibrary|LineTraceMultiforObjects (+ _returnvalue "0, 0,160.000000") (- _returnvalue "0, 0,96.000000") (Utilities|Array|MakeArray "ObjectTypeQuery1") false 0 "None" true))
      (bind _returnvalue_3 (Class|BuildableFunctionLibrary|HasStaticGroundinHitResults _outhits))
      (if _returnvalue_3
        _
        (else
          (return (Utilities|String|ToString(Text) (Variables|Default|GetError_MustConnectToLandscapeOrSocket)) "Fail")))))
  (return _failedmessage _returnvalue_2))
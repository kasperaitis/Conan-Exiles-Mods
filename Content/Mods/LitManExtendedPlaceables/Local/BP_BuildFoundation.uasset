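; Foundation building piece from the LitManExtendedPlaceables mod that overrides CanBePlaced to require ground or structural support.
; A vertical box trace looks for static ground, and a short downward overlap sweep looks for foundations, pillars, ceilings, altars or thrall converters.
; With either support it returns the parent's result, otherwise it fails with a missing-landscape error.
; Clients skip the support check while MIsLoading is set.
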(event EventBeginPlay)

(event Collision|EventActorBeginOverlap
  (params (OtherActor :type Actor%20Object%20Reference)))

(event EventTick
  (params (DeltaSeconds :type Float%20%28single-precision%29)))

(fn ConstructionScript
  (|CallParentFunction))

(fn CanbePlaced
  (params (AttachTo :type Buildable%20Base%20Object%20Reference) (InstanceIndex :type Integer))
  (bind _checkforlandscapeboxchecker (Variables|Default|GetCheckForLandscapeBoxChecker))
  (bind _returnvalue (Transformation|GetWorldLocation _checkforlandscapeboxchecker))
  (bind (_x _y _z) (Math|Vector|BreakVector _returnvalue))
  (bind (_x_2 _y_2 _z_2) (Math|Vector|BreakVector _returnvalue))
  (bind (_failedmessage _returnvalue_2) (|CallParentFunction AttachTo InstanceIndex))
  (if (Networking|IsServer)
    (if (< (Math|Conversions|ToInteger(Byte) _returnvalue_2) (Math|Conversions|ToInteger(Byte) (Utilities|Enum|LiteralenumECanBePlacedResult "Fail")))
      _
      (else
        (return _failedmessage _returnvalue_2)))
    (elif (Variables|Default|Getm_IsLoading)
      (if (< (Math|Conversions|ToInteger(Byte) _returnvalue_2) (Math|Conversions|ToInteger(Byte) (Utilities|Enum|LiteralenumECanBePlacedResult "Fail")))
        (return "" "Success")
        (else
          (return _failedmessage _returnvalue_2)))
      (else
        _)))
  (Utilities|Array|Clear (Variables|Default|GetFoundFoundation))
  (bind _outhits (Class|KismetSystemLibrary|BoxTraceMulti (Math|Vector|MakeVector _x_2 _y_2 (+ _z_2 128.0)) (Math|Vector|MakeVector _x _y (- _z 32.0)) (Variables|/Script/Engine.BoxComponent|GetBoxExtent _checkforlandscapeboxchecker) (Transformation|GetWorldRotation _checkforlandscapeboxchecker) "TraceTypeQuery1" false 0 "None" true))
  (bind _returnvalue_3 (Class|BuildableFunctionLibrary|HasStaticGroundinHitResults _outhits))
  (LocalVariables|SetHasFoundLandscape _returnvalue_3)
  (bind _foundoverlaps (CallFunction|CheckforOverlappingStructure (Variables|Default|GetCheckForValidBuildingSupport) 32.0 (Utilities|Array|MakeArray "/Game/Systems/Building/BP_BuildFoundation.BP_BuildFoundation_C" "/Game/Systems/Building/BP_BuildPillar.BP_BuildPillar_C" "/Game/Systems/Building/BP_BuildCeiling.BP_BuildCeiling_C" "/Game/Systems/Building/Placeables/BP_PL_Altar.BP_PL_Altar_C" "/Game/Systems/Building/Placeables/BP_PL_CraftingStation_ThrallConverter.BP_PL_CraftingStation_ThrallConverter_C")))
  (if (or _foundoverlaps (LocalVariables|GetHasFoundLandscape))
    (return _failedmessage _returnvalue_2)
    (else
      (return (Utilities|String|ToString(Text) (Variables|Default|GetError_CouldntFindLandscape)) "Fail"))))
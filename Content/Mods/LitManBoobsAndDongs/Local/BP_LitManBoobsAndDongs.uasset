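; Mod controller Blueprint for the LitManBoobsAndDongs mod for Conan Exiles, mostly an unfinished scaffold.
; ModDataTableOperations makes two data table merge calls, referencing the spawn and equipment template tables, each with only one table argument set.
; BeginPlay, Tick and the construction script are empty.
; Disconnected experiments print character skeleton and mesh names and probe the male AnimBP and AnimDynamics settings for body physics, but never run.
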(event EventBeginPlay)

(event EventTick
  (params (DeltaSeconds :type Float%20%28single-precision%29)))

(fn ConstructionScript)

(fn ModDataTableOperations
  (Class|ModController|MergeDataTables "/Game/Systems/SpawnTable/SpawnDataTable.SpawnDataTable")
  (Class|ModController|MergeDataTables 0 "/Game/Systems/SpawnTable/EquipmentTemplateDataTable.EquipmentTemplateDataTable"))
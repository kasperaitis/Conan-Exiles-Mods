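; LitManDurability mod Blueprint that scales down the server's durability and shield durability multipliers.
; On BeginPlay it waits briefly, then divides both server-settings values in place by a fixed factor, so the change is relative to the configured values.
; Debug prints of the multipliers are left disconnected, and the construction script, data table operations and rep-notify functions are empty.
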(event EventBeginPlay
  (bind _returnvalue (|GetServerSettings))
  (bind _returnvalue_2 (|GetServerSettings))
  (Utilities|FlowControl|Delay 1.0)
  (bind _output_get (Variables|/Script/ConanSandbox.ServerSettings|SetDurabilityMultiplier _returnvalue (/ (Variables|/Script/ConanSandbox.ServerSettings|GetDurabilityMultiplier _returnvalue_2) 1e+01)))
  (bind _output_get_2 (Variables|/Game/Systems/BP_ServerSettings.BP_ServerSettings_C|SetShieldDurabilityMultiplier _returnvalue (/ (Variables|/Game/Systems/BP_ServerSettings.BP_ServerSettings_C|GetShieldDurabilityMultiplier _returnvalue_2) 1e+01))))

(event EventTick
  (params (DeltaSeconds :type Float%20%28single-precision%29)))

(fn ConstructionScript)

(fn ModDataTableOperations)

(fn OnRepLitManModDurabilityTemp)
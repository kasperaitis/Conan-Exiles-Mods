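; Combat durability helper that wears down weapons, shields and tools through ModifyDurability when their owner is allowed to lose durability.
; Weapon loss scales with the server multiplier and skips one hardcoded item template.
; Shield loss varies by projectile or melee hit, scales with server settings, and can be randomly negated by the Encumberance_40 perk.
; Tool loss ignores server settings, using normal or heavy amounts depending on CanMine.
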(fn AffectDurabilityWeapon
  (params (Weapon :type Base%20Weapon%20Object%20Reference))
  (bind _output_get (LocalVariables|Setlocal%20Weapon Weapon))
  (if (not (== (Variables|/Script/ConanSandbox.GameItem|GetTemplateID (Variables|/Script/ConanSandbox.InventoryItemBase|GetOwnerItem _output_get)) 51468))
    (if (> (Class|GameItem|GetFloatStat (Variables|/Script/ConanSandbox.InventoryItemBase|GetOwnerItem (LocalVariables|Getlocal%20Weapon)) "MaxDurability") 0.0) ; Durability will only be tested if the weapon has \nmore than zero max durability
      (if (Variables|/Game/Characters/BaseBPCombat.BaseBPCombat_C|GetCanLoseDurabilityWeapon (Variables|/Game/Items/Weapons/BaseHitActor.BaseHitActor_C|GetCharacterOwner (LocalVariables|Getlocal%20Weapon)))
        (Class|GameItem|ModifyDurability (Variables|/Script/ConanSandbox.InventoryItemBase|GetOwnerItem (LocalVariables|Getlocal%20Weapon)) (* -1.0 (/ (Class|ServerSettings|GetDurabilityMultiplier (|GetServerSettings)) 1e+01)))))))

(fn AffectDurabilityShield
  (params (ShieldOwner :type Actor%20Object%20Reference) (ProjectileHit :type Boolean))
  (LocalVariables|Setlocal%20ShieldOwner ShieldOwner)
  (LocalVariables|Setlocal%20ProjectileHit ProjectileHit)
  (bind _shieldobject (Class|IsBaseBPCombatInterface|GetActiveShield(Message) (LocalVariables|Getlocal%20ShieldOwner)))
  (bind _asbase_weapon (Utilities|Casting|CastToBaseWeapon _shieldobject))
  (if (Variables|/Game/Characters/BaseBPCombat.BaseBPCombat_C|GetCanLoseDurabilityShield (Variables|/Game/Items/Weapons/BaseHitActor.BaseHitActor_C|GetCharacterOwner _asbase_weapon))
    (Utilities|FlowControl|Sequence
      (:then_0
        (bind _asi_perk_system_owner_interface (Utilities|Casting|CastToI_PerkSystemOwnerInterface (Variables|/Game/Items/Weapons/BaseHitActor.BaseHitActor_C|GetCharacterOwner _asbase_weapon))
          (:then
            (bind _perksysteminterface (Default|GetPerkSystem _asi_perk_system_owner_interface))
            (bind _hasperk (Default|HasPerk _perksysteminterface "Encumberance_40"))
            (if _hasperk
              (bind _modifier (Default|GetPerksGotHitDurabilityModifier _perksysteminterface))
              (LocalVariables|Setlocal%20DurabilityLossChanceFromPerks _modifier)
              (else
                (LocalVariables|Setlocal%20DurabilityLossChanceFromPerks 0.0 :!label _label))))
          (:CastFailed
            (goto _label))))
      (:then_1
        (if (not (< (Math|Random|RandomFloat) (LocalVariables|Getlocal%20DurabilityLossChanceFromPerks)))
          (Class|GameItem|ModifyDurability (Variables|/Script/ConanSandbox.InventoryItemBase|GetOwnerItem _asbase_weapon) (* (Class|ServerSettings|GetDurabilityMultiplier (|GetServerSettings)) (* (* (select (LocalVariables|Getlocal%20ProjectileHit) (LocalVariables|GetShieldProjectileDurabilityDamagePerHit) (LocalVariables|GetShieldMeleeDurabilityDamagePerHit)) (/ (Variables|/Game/Systems/BP_ServerSettings.BP_ServerSettings_C|GetShieldDurabilityMultiplier (|GetServerSettings)) 1e+01)) -1.0))))))))

(fn AffectDurabilityTool
  (params (Weapon :type Base%20Weapon%20Object%20Reference) (CanMine :type Boolean))
  (LocalVariables|Setlocal%20Weapon Weapon)
  (if (> (Class|GameItem|GetFloatStat (Variables|/Script/ConanSandbox.InventoryItemBase|GetOwnerItem (LocalVariables|Getlocal%20Weapon)) "MaxDurability") 0.0) ; Durability will only be tested if the weapon has \nmore than zero max durability
    (if (Variables|/Game/Characters/BaseBPCombat.BaseBPCombat_C|GetCanLoseDurabilityWeapon (Variables|/Game/Items/Weapons/BaseHitActor.BaseHitActor_C|GetCharacterOwner (LocalVariables|Getlocal%20Weapon)))
      (if CanMine
        (Class|GameItem|ModifyDurability (Variables|/Script/ConanSandbox.InventoryItemBase|GetOwnerItem (LocalVariables|Getlocal%20Weapon)) (* -1.0 (/ (LocalVariables|Getlocal%20DurabilityLossNormal) 1e+01)))
        (else
          (Class|GameItem|ModifyDurability (Variables|/Script/ConanSandbox.InventoryItemBase|GetOwnerItem (LocalVariables|Getlocal%20Weapon)) (* -1.0 (/ (LocalVariables|Getlocal%20DurabilityLossHeavy) 1e+01))))))))
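; Mod Blueprint that shrinks the thrall placement exclusion radius so thralls can be placed closer together.
; Shortly after BeginPlay it checks the ThrallExclusionRadius server setting and, on the server only, lowers it if it still holds the expected starting value, leaving other values untouched.
; Unconnected leftover nodes hold debug prints and persistence-dirty calls; ModDataTableOperations is empty.
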(event EventBeginPlay
  (Utilities|FlowControl|Delay 1.0)
  (if (== (Variables|/Game/Systems/BP_ServerSettings.BP_ServerSettings_C|GetThrallExclusionRadius (|GetServerSettings)) 5e+02)
    (if (Networking|IsServer)
      (Variables|/Game/Systems/BP_ServerSettings.BP_ServerSettings_C|SetThrallExclusionRadius (|GetServerSettings) 1e+02))))

(event EventTick
  (params (DeltaSeconds :type Float%20%28single-precision%29)))

(fn ConstructionScript)

(fn ModDataTableOperations)
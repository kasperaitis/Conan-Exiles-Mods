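; Test-mod actor component for Conan that applies a pubic hair texture to players and humanoid NPCs at full nudity.
; After delayed BeginPlay it applies the texture and rebinds on player layout changes or NPC mesh initialization.
; A stored ID, or random first pick, indexes gendered DataTables to set the lower-body dynamic materials' texture parameter, then dirties persistence or inventory.
; Debug prints remain; the character-creation widget hook is never bound.
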(event Custom|PubicHairChar
  (CallFunction|SetPubicHairChar (stale EventBeginPlay _asbase_player_char)))

(event Custom|CharacterCreation
  (params (module :type GUI%20Module%20Object%20Reference) (isActive :type Boolean))
  (if isActive
    (bind _foundwidgets (Widget|GetAllWidgetsOfClass "/Game/UI/CharacterCreation/W_CharacterCreation_Main.W_CharacterCreation_Main_C" false))
    (for _array_element _foundwidgets
      (Utilities|IsValid "/Game/Mods/LitManTestMod/LitMan_W_Physique.LitMan_W_Physique"
        (:Is%20Valid
          _)
        (:Is%20Not%20Valid
          (bind _returnvalue (UserInterface|CreateWidget "/Game/Mods/LitManTestMod/LitMan_W_Physique.LitMan_W_Physique_C" (Game|GetPlayerController 0)))
          (Variables|Default|SetLitManWidget _returnvalue)))
      (CallFunction|AddWidget _array_element))))

(event Custom|PubickHairGUI
  (CallFunction|SetPubicHairChar (stale EventBeginPlay _asbase_humanoid_npc_2)))

(event Custom|PubicHairNPC
  (CallFunction|SetPubicHairNPC (stale EventBeginPlay _asbase_humanoid_npc)))

(event Custom|AddWidget
  (params (parent :type W%20Character%20Creation%20Main%20Object%20Reference))
  (bind _returnvalue (Class|VerticalBox|AddChildtoVerticalBox (Variables|/Game/UI/CharacterCreation/W_CharacterCreation_Main.W_CharacterCreation_Main_C|GetMainPanel_Buttons parent) (Variables|Default|GetLitManWidget)))
  (Layout|GridSlot|SetVerticalAlignment _returnvalue "VAlign_Bottom")
  (Layout|GridSlot|SetHorizontalAlignment _returnvalue "HAlign_Fill")
  (Class|VerticalBoxSlot|SetSize _returnvalue (Utilities|Struct|MakeSlateChildSize 1.0 "Automatic"))
  (Layout|BorderSlot|SetPadding _returnvalue (Utilities|Struct|MakeMargin 0.0 2e+01 0.0 0.0) :!class /Script/UMG.VerticalBoxSlot))

(event EventBeginPlay
  (Utilities|FlowControl|Delay 2.0)
  (Utilities|FlowControl|Sequence
    (:then_0
      (bind _asbase_player_char (Utilities|Casting|CastToBasePlayerChar (Components|GetOwner)))
      (Utilities|FlowControl|Delay 2.0)
      (CallFunction|SetPubicHairChar _asbase_player_char)
      (EventDispatchers|BindEventtoSignalCharacterLayoutChange _asbase_player_char (delegate Custom|PubicHairChar)))
    (:then_1
      (bind _asbase_humanoid_npc (Utilities|Casting|CastToBaseHumanoidNPC (Components|GetOwner)))
      (Utilities|FlowControl|Delay 2.0)
      (CallFunction|SetPubicHairNPC _asbase_humanoid_npc)
      (EventDispatchers|BindEventtoOnSkeletalMeshInitialized (Actor|GetComponentbyClass (Components|GetOwner) "/Game/Characters/BP_CharacterCustomizationComponent.BP_CharacterCustomizationComponent_C") (delegate Custom|PubicHairNPC)))
    (:then_2
      (bind _asw_uicharacter_display (Utilities|Casting|CastToW_UICharacterDisplay))
      (CallFunction|SetPubicHairChar (Components|GetOwner))
      (bind _asbase_humanoid_npc_2 (Utilities|Casting|CastToBaseHumanoidNPC _asw_uicharacter_display))
      (EventDispatchers|BindEventtoSignalThrallLayoutChange (delegate Custom|PubickHairGUI)))))

(event EventTick
  (params (DeltaSeconds :type Float%20%28single-precision%29)))

(fn OnRepPubicHairTexture)

(fn SetPubicHairChar
  (params (PlayerChar :type Actor%20Object%20Reference))
  (bind _returnvalue (Utilities|Name|MakeLiteralName "Bodyhair Texture"))
  (if (Utilities|Enum|Equal(Enum) (CallFunction|GetClampedNudityLevel) "Full")
    (bind _asbase_player_char (Utilities|Casting|CastToBasePlayerChar PlayerChar))
    (bind _layout (Default|GetCharacterLayout _asbase_player_char))
    (bind (_array_element _array_index) (Utilities|Array|ForEachLoopwithBreak (Variables|/Script/ConanSandbox.CharacterCustomizationComponent|GetSkeletalMeshes (Variables|/Game/Characters/BasePlayerChar.BasePlayerChar_C|GetBP_CharacterCustomizationComponent _asbase_player_char)) :!label _label)
      (:LoopBody
        (Variables|Default|SetPlayerOwner _asbase_player_char)
        (Development|PrintString (Utilities|GetDisplayName _array_element) true true "(R=1.000000,G=0.839612,B=0.000000,A=1.000000)" 1e+01)
        (Development|PrintString (Utilities|String|ToString(Integer) _array_index) true true "(R=0.000000,G=1.000000,B=0.337630,A=1.000000)" 1e+01)
        (if (== _array_index 7)
          (bind _output_get (Variables|Default|SetBPCLowerbody _array_element))
          (if (Utilities|Struct|BreakCharacterBoolParameters (.BoolParams (Utilities|Struct|BreakCharacterLayout _layout)))
            (bind _outrownames (DataTable|GetDataTableRowNames "/Game/Mods/LitManTestMod/LitMan_DT_FemalePubicHair.LitMan_DT_FemalePubicHair"))
            (Variables|Default|SetRandomInt (Math|Random|RandomIntegerinRange 1 (Utilities|Array|Length _outrownames)))
            (if (!= (Variables|Default|GetPubicHairID) -1)
              (bind _rowname (CallFunction|LitManGetRowNamesfromIndex "/Game/Mods/LitManTestMod/LitMan_DT_FemalePubicHair.LitMan_DT_FemalePubicHair" (Variables|Default|GetPubicHairID)))
              (bind _returnvalue_2 (Utilities|GetDataTableRow "/Game/Mods/LitManTestMod/LitMan_DT_FemalePubicHair.LitMan_DT_FemalePubicHair" _rowname)
                (:then
                  (Variables|Default|SetPubicHairTexture (.texture (Utilities|Struct|BreakLitMan_STR_PubicHair _returnvalue_2)))
                  (Class|PersistenceComponent|SetDirty (Variables|/Game/Characters/BasePlayerChar.BasePlayerChar_C|GetConanCharacterPersistence (Variables|Default|GetPlayerOwner)) true 0.2)))
              (else
                (bind _rowname_2 (CallFunction|LitManGetRowNamesfromIndex "/Game/Mods/LitManTestMod/LitMan_DT_FemalePubicHair.LitMan_DT_FemalePubicHair" (Variables|Default|GetRandomInt)))
                (bind _returnvalue_3 (Utilities|GetDataTableRow "/Game/Mods/LitManTestMod/LitMan_DT_FemalePubicHair.LitMan_DT_FemalePubicHair" _rowname_2)
                  (:then
                    (Variables|Default|SetPubicHairID (.id (Utilities|Struct|BreakLitMan_STR_PubicHair _returnvalue_3)))
                    (Variables|Default|SetPubicHairTexture (.texture (Utilities|Struct|BreakLitMan_STR_PubicHair _returnvalue_3)))
                    (Class|PersistenceComponent|SetDirty (Variables|/Game/Characters/BasePlayerChar.BasePlayerChar_C|GetConanCharacterPersistence (Variables|Default|GetPlayerOwner)) true 0.2)))))
            (else
              (bind _outrownames_2 (DataTable|GetDataTableRowNames "/Game/Mods/LitManTestMod/LitMan_DT_MalePubicHair.LitMan_DT_MalePubicHair"))
              (Variables|Default|SetRandomInt (Math|Random|RandomIntegerinRange 1 (Utilities|Array|Length _outrownames_2)))
              (if (!= (Variables|Default|GetPubicHairID) -1)
                (bind _rowname_3 (CallFunction|LitManGetRowNamesfromIndex "/Game/Mods/LitManTestMod/LitMan_DT_MalePubicHair.LitMan_DT_MalePubicHair" (Variables|Default|GetPubicHairID)))
                (bind _returnvalue_4 (Utilities|GetDataTableRow "/Game/Mods/LitManTestMod/LitMan_DT_MalePubicHair.LitMan_DT_MalePubicHair" _rowname_3)
                  (:then
                    (Variables|Default|SetPubicHairTexture (.texture (Utilities|Struct|BreakLitMan_STR_PubicHair _returnvalue_4)))
                    (Class|PersistenceComponent|SetDirty (Variables|/Game/Characters/BasePlayerChar.BasePlayerChar_C|GetConanCharacterPersistence (Variables|Default|GetPlayerOwner)) true 0.2)))
                (else
                  (bind _rowname_4 (CallFunction|LitManGetRowNamesfromIndex "/Game/Mods/LitManTestMod/LitMan_DT_MalePubicHair.LitMan_DT_MalePubicHair" (Variables|Default|GetRandomInt)))
                  (bind _returnvalue_5 (Utilities|GetDataTableRow "/Game/Mods/LitManTestMod/LitMan_DT_MalePubicHair.LitMan_DT_MalePubicHair" _rowname_4)
                    (:then
                      (Variables|Default|SetPubicHairID (.id (Utilities|Struct|BreakLitMan_STR_PubicHair _returnvalue_5)))
                      (Variables|Default|SetPubicHairTexture (.texture (Utilities|Struct|BreakLitMan_STR_PubicHair _returnvalue_5)))
                      (Class|PersistenceComponent|SetDirty (Variables|/Game/Characters/BasePlayerChar.BasePlayerChar_C|GetConanCharacterPersistence (Variables|Default|GetPlayerOwner)) true 0.2)))))))
          (for _array_element_2 (Rendering|Material|GetMaterials _output_get)
            ;[1 1 1] Get materials
            (bind _asmaterial_instance_dynamic (Utilities|Casting|CastToMaterialInstanceDynamic _array_element_2)
              (:then
                (bind _output_get_2 (Variables|Default|SetMID _asmaterial_instance_dynamic))
                (Rendering|Material|GetTextureParameterValue _output_get_2 _returnvalue :!class /Script/Engine.MaterialInstanceDynamic)
                (Development|PrintString (Utilities|String|Append "Char Asigned Texture: " (Utilities|GetDisplayName (Variables|Default|GetPubicHairTexture))) true true "(R=0.000000,G=0.660000,B=1.000000,A=1.000000)" 1e+01)
                (Rendering|Material|SetTextureParameterValue (Variables|Default|GetMID) _returnvalue (Variables|Default|GetPubicHairTexture)))
              (:CastFailed
                (Development|PrintString "Cast Failed"))))
          (goto _label Break)))
      (:Completed
        (Rendering|Material|SetMaterial (Variables|Default|GetBPCLowerbody) 7 (Variables|Default|GetMID))))))

(fn SetPubicHairNPC
  (params (HumanoidNPC :type Actor%20Object%20Reference))
  (bind _returnvalue (Utilities|Name|MakeLiteralName "Bodyhair Texture"))
  (if (Utilities|Enum|Equal(Enum) (CallFunction|GetClampedNudityLevel) "Full")
    (bind _asbase_humanoid_npc (Utilities|Casting|CastToBaseHumanoidNPC HumanoidNPC))
    (bind _layout (Default|GetCharacterLayout _asbase_humanoid_npc))
    (bind (_array_element _array_index) (Utilities|Array|ForEachLoopwithBreak (Variables|/Script/ConanSandbox.CharacterCustomizationComponent|GetSkeletalMeshes (Variables|/Game/Characters/NPCs/Humanoid/BaseHumanoidNPC.BaseHumanoidNPC_C|GetBP_CharacterCustomizationComponent _asbase_humanoid_npc)) :!label _label)
      (:LoopBody
        (Variables|Default|SetNPCOwner _asbase_humanoid_npc)
        (if (== _array_index 7)
          (bind _output_get (Variables|Default|SetBPCLowerbody _array_element))
          (if (Utilities|Struct|BreakCharacterBoolParameters (.BoolParams (Utilities|Struct|BreakCharacterLayout _layout)))
            (bind _outrownames (DataTable|GetDataTableRowNames "/Game/Mods/LitManTestMod/LitMan_DT_FemalePubicHair.LitMan_DT_FemalePubicHair"))
            (Variables|Default|SetRandomInt (Math|Random|RandomIntegerinRange 1 (Utilities|Array|Length _outrownames)))
            (if (!= (Variables|Default|GetPubicHairID) -1)
              (bind _rowname (CallFunction|LitManGetRowNamesfromIndex "/Game/Mods/LitManTestMod/LitMan_DT_FemalePubicHair.LitMan_DT_FemalePubicHair" (Variables|Default|GetPubicHairID)))
              (bind _returnvalue_2 (Utilities|GetDataTableRow "/Game/Mods/LitManTestMod/LitMan_DT_FemalePubicHair.LitMan_DT_FemalePubicHair" _rowname)
                (:then
                  (Variables|Default|SetPubicHairTexture (.texture (Utilities|Struct|BreakLitMan_STR_PubicHair _returnvalue_2)))))
              (else
                (bind _rowname_2 (CallFunction|LitManGetRowNamesfromIndex "/Game/Mods/LitManTestMod/LitMan_DT_FemalePubicHair.LitMan_DT_FemalePubicHair" (Variables|Default|GetRandomInt)))
                (bind _returnvalue_3 (Utilities|GetDataTableRow "/Game/Mods/LitManTestMod/LitMan_DT_FemalePubicHair.LitMan_DT_FemalePubicHair" _rowname_2)
                  (:then
                    (Variables|Default|SetPubicHairID (.id (Utilities|Struct|BreakLitMan_STR_PubicHair _returnvalue_3)))
                    (Variables|Default|SetPubicHairTexture (.texture (Utilities|Struct|BreakLitMan_STR_PubicHair _returnvalue_3)))
                    (Class|PersistenceComponent|SetDirty (Variables|/Game/Characters/BaseBPChar.BaseBPChar_C|GetEquipmentInventory (Variables|Default|GetNPCOwner)) true 0.2)))))
            (else
              (bind _outrownames_2 (DataTable|GetDataTableRowNames "/Game/Mods/LitManTestMod/LitMan_DT_MalePubicHair.LitMan_DT_MalePubicHair"))
              (Variables|Default|SetRandomInt (Math|Random|RandomIntegerinRange 1 (Utilities|Array|Length _outrownames_2)))
              (if (!= (Variables|Default|GetPubicHairID) -1)
                (bind _rowname_3 (CallFunction|LitManGetRowNamesfromIndex "/Game/Mods/LitManTestMod/LitMan_DT_MalePubicHair.LitMan_DT_MalePubicHair" (Variables|Default|GetPubicHairID)))
                (bind _returnvalue_4 (Utilities|GetDataTableRow "/Game/Mods/LitManTestMod/LitMan_DT_MalePubicHair.LitMan_DT_MalePubicHair" _rowname_3)
                  (:then
                    (Variables|Default|SetPubicHairTexture (.texture (Utilities|Struct|BreakLitMan_STR_PubicHair _returnvalue_4)))
                    (Class|PersistenceComponent|SetDirty (Variables|/Game/Characters/BaseBPChar.BaseBPChar_C|GetEquipmentInventory (Variables|Default|GetNPCOwner)) true 0.2)))
                (else
                  (bind _rowname_4 (CallFunction|LitManGetRowNamesfromIndex "/Game/Mods/LitManTestMod/LitMan_DT_MalePubicHair.LitMan_DT_MalePubicHair" (Variables|Default|GetRandomInt)))
                  (bind _returnvalue_5 (Utilities|GetDataTableRow "/Game/Mods/LitManTestMod/LitMan_DT_MalePubicHair.LitMan_DT_MalePubicHair" _rowname_4)
                    (:then
                      (Variables|Default|SetPubicHairID (.id (Utilities|Struct|BreakLitMan_STR_PubicHair _returnvalue_5)))
                      (Variables|Default|SetPubicHairTexture (.texture (Utilities|Struct|BreakLitMan_STR_PubicHair _returnvalue_5)))
                      (Class|PersistenceComponent|SetDirty (Variables|/Game/Characters/BaseBPChar.BaseBPChar_C|GetEquipmentInventory (Variables|Default|GetNPCOwner)) true 0.2)))))))
          (for _array_element_2 (Rendering|Material|GetMaterials _output_get)
            ;[1 1 1] Get materials
            (bind _asmaterial_instance_dynamic (Utilities|Casting|CastToMaterialInstanceDynamic _array_element_2)
              (:then
                (bind _output_get_2 (Variables|Default|SetMID _asmaterial_instance_dynamic))
                (Rendering|Material|GetTextureParameterValue _output_get_2 _returnvalue :!class /Script/Engine.MaterialInstanceDynamic)
                (Development|PrintString (Utilities|String|Append "NPC Asigned Texture: " (Utilities|GetDisplayName (Variables|Default|GetPubicHairTexture))) true true "(R=0.000000,G=0.660000,B=1.000000,A=1.000000)" 1e+01)
                (Rendering|Material|SetTextureParameterValue (Variables|Default|GetMID) _returnvalue (Variables|Default|GetPubicHairTexture))
                (Class|PersistenceComponent|SetDirty (Variables|/Game/Characters/BaseBPChar.BaseBPChar_C|GetEquipmentInventory (Variables|Default|GetNPCOwner)) true 0.2))
              (:CastFailed
                (Development|PrintString "Cast Failed"))))
          (goto _label Break)))
      (:Completed
        (Rendering|Material|SetMaterial (Variables|Default|GetBPCLowerbody) 0 (Variables|Default|GetMID))))))

(fn LitManGetRowNamesfromIndex
  (params (DataTable :type Data%20Table%20Object%20Reference) (RowIndex :type Integer))
  (bind _outrownames (DataTable|GetDataTableRowNames DataTable))
  (if (not (Utilities|Array|IsValidIndex _outrownames RowIndex))
    (return "None")
    (else
      (return (Utilities|Array|Get(acopy) _outrownames (- RowIndex 1))))))
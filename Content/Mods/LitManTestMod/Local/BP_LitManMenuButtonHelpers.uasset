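; Helper Blueprint in LitManTestMod that adds new menu buttons next to existing ones.
; CreateAndInsertButton creates a W_ButtonNormal with the source button's style, font and colors, sets its label and window, then, if the parent is a VerticalBox, splices it into keyboard navigation above the source.
; InsertWidgetAtIndex places it at the source's index by removing trailing children and re-adding them after it in original order.
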(fn InsertWidgetatIndex
  (params (Parent :type Panel%20Widget%20Object%20Reference) (WidgetToInsert :type Widget%20Object%20Reference) (TargetIndex :type Integer))
  (bind _output_get (LocalVariables|SetLocLoopCounter (- (Class|PanelWidget|GetChildrenCount Parent) 1)))
  (if (>= _output_get TargetIndex) :!label _label
    (Utilities|Array|Add (LocalVariables|GetTempWidgets) (Class|PanelWidget|GetChildat Parent (LocalVariables|GetLocLoopCounter)))
    (Class|PanelWidget|RemoveChild Parent (Class|PanelWidget|GetChildat Parent (LocalVariables|GetLocLoopCounter)))
    (Math|Integer|DecrementInt (LocalVariables|GetLocLoopCounter)
      (:%20%20
        (goto _label)))
    (else
      (Widget|Panel|AddChild Parent WidgetToInsert)
      (bind _arrayelement (Utilities|Array|ReverseforEachLoop (LocalVariables|GetTempWidgets))
        (:LoopBody
          (Widget|Panel|AddChild Parent _arrayelement))))))

(fn CreateandInsertButton
  (params (SourceButton :type W%20Button%20Normal%20Object%20Reference) (ButtonLabel :type Text) (WindowRoot :type Window%20Root%20Object%20Reference))
  (Utilities|FlowControl|Sequence
    (:then_0
      (bind _output_get (LocalVariables|SetLoc_ButtonToCopy SourceButton))
      (bind _returnvalue (UserInterface|CreateWidget "/Game/UI/Framework/W_ButtonNormal.W_ButtonNormal_C" (Widget|GetOwningPlayer _output_get)))
      (LocalVariables|SetLoc_NewButton _returnvalue))
    (:then_1
      (Variables|/Script/ConanSandbox.FCButton|SetStyle (LocalVariables|GetLoc_NewButton) (Variables|/Script/ConanSandbox.FCButton|GetStyle (LocalVariables|GetLoc_ButtonToCopy)))
      (Utilities|Struct|SetmembersinSlateColor (Variables|/Script/ConanSandbox.FCButton|GetFontColor (LocalVariables|GetLoc_NewButton)) (.SpecifiedColor (Utilities|Struct|BreakSlateColor (Variables|/Script/ConanSandbox.FCButton|GetFontColor (LocalVariables|GetLoc_ButtonToCopy)))) (.ColorUseRule (Utilities|Struct|BreakSlateColor (Variables|/Script/ConanSandbox.FCButton|GetFontColor (LocalVariables|GetLoc_ButtonToCopy)))))
      (Utilities|Struct|SetmembersinSlateColor (Variables|/Script/ConanSandbox.FCButton|GetHoveredFontColor (LocalVariables|GetLoc_NewButton)) (.SpecifiedColor (Utilities|Struct|BreakSlateColor (Variables|/Script/ConanSandbox.FCButton|GetHoveredFontColor (LocalVariables|GetLoc_ButtonToCopy)))) (.ColorUseRule (Utilities|Struct|BreakSlateColor (Variables|/Script/ConanSandbox.FCButton|GetHoveredFontColor (LocalVariables|GetLoc_ButtonToCopy)))))
      (Utilities|Struct|SetmembersinSlateColor (Variables|/Script/ConanSandbox.FCButton|GetPressedFontColor (LocalVariables|GetLoc_NewButton)) (.SpecifiedColor (Utilities|Struct|BreakSlateColor (Variables|/Script/ConanSandbox.FCButton|GetPressedFontColor (LocalVariables|GetLoc_ButtonToCopy)))) (.ColorUseRule (Utilities|Struct|BreakSlateColor (Variables|/Script/ConanSandbox.FCButton|GetPressedFontColor (LocalVariables|GetLoc_ButtonToCopy)))))
      (Utilities|Struct|SetmembersinSlateColor (Variables|/Script/ConanSandbox.FCButton|GetPressedHoveredFontColor (LocalVariables|GetLoc_NewButton)) (.SpecifiedColor (Utilities|Struct|BreakSlateColor (Variables|/Script/ConanSandbox.FCButton|GetPressedHoveredFontColor (LocalVariables|GetLoc_ButtonToCopy)))) (.ColorUseRule (Utilities|Struct|BreakSlateColor (Variables|/Script/ConanSandbox.FCButton|GetPressedHoveredFontColor (LocalVariables|GetLoc_ButtonToCopy)))))
      (Utilities|Struct|SetmembersinSlateFontInfo (Variables|/Script/ConanSandbox.FCButton|GetLabelFont (LocalVariables|GetLoc_NewButton)) (.FontObject (Utilities|Struct|BreakSlateFontInfo (Variables|/Script/ConanSandbox.FCButton|GetLabelFont (LocalVariables|GetLoc_ButtonToCopy)))) (.FontMaterial (Utilities|Struct|BreakSlateFontInfo (Variables|/Script/ConanSandbox.FCButton|GetLabelFont (LocalVariables|GetLoc_ButtonToCopy)))) (.OutlineSettings (Utilities|Struct|BreakSlateFontInfo (Variables|/Script/ConanSandbox.FCButton|GetLabelFont (LocalVariables|GetLoc_ButtonToCopy)))) (.TypefaceFontName (Utilities|Struct|BreakSlateFontInfo (Variables|/Script/ConanSandbox.FCButton|GetLabelFont (LocalVariables|GetLoc_ButtonToCopy)))) (.Size (Utilities|Struct|BreakSlateFontInfo (Variables|/Script/ConanSandbox.FCButton|GetLabelFont (LocalVariables|GetLoc_ButtonToCopy)))))
      (Variables|/Script/ConanSandbox.FCButton|SetLabel (LocalVariables|GetLoc_NewButton) ButtonLabel))
    (:then_2
      (Class|RootWidget|SetWindow (LocalVariables|GetLoc_NewButton) WindowRoot)
      (bind _asvertical_box (Utilities|Casting|CastToVerticalBox (Widget|GetParent (LocalVariables|GetLoc_ButtonToCopy)))
        (:then
          (Variables|/Script/ConanSandbox.RootWidget|SetKeyNavAbove (LocalVariables|GetLoc_NewButton) (Variables|/Script/ConanSandbox.RootWidget|GetKeyNavAbove (LocalVariables|GetLoc_ButtonToCopy)))
          (Variables|/Script/ConanSandbox.RootWidget|SetKeyNavBelow (LocalVariables|GetLoc_NewButton) (LocalVariables|GetLoc_ButtonToCopy))
          (Variables|/Script/ConanSandbox.RootWidget|SetKeyNavBelow (Variables|/Script/ConanSandbox.RootWidget|GetKeyNavAbove (LocalVariables|GetLoc_ButtonToCopy)) (LocalVariables|GetLoc_NewButton))
          (Variables|/Script/ConanSandbox.RootWidget|SetKeyNavAbove (LocalVariables|GetLoc_ButtonToCopy) (LocalVariables|GetLoc_NewButton))
          (Widget|Panel|InsertWidgetatIndex 0 _asvertical_box (LocalVariables|GetLoc_NewButton) (Class|PanelWidget|GetChildIndex _asvertical_box (LocalVariables|GetLoc_ButtonToCopy)))
          (return (LocalVariables|GetLoc_NewButton)))
        (:CastFailed
          (return 0))))))
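; LitManTestMod's mod Blueprint, which merges spawn and equipment template data tables and holds logic to inject a custom physique widget into character creation.
; When active, the CharacterCreation event creates a LitMan_W_Physique for each main character creation widget found and adds it to that widget's MainPanelButtons.
; The signal binding for that event is disconnected and BeginPlay is empty, so nothing in this graph triggers the injection.
; The UI module table merge is also disconnected.
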(event Custom|CharacterCreation
  (params (module :type GUI%20Module%20Object%20Reference) (isActive :type Boolean))
  (if isActive
    (bind _foundwidgets (Widget|GetAllWidgetsOfClass "/Game/UI/CharacterCreation/W_CharacterCreation_Main.W_CharacterCreation_Main_C" false))
    (for _array_element _foundwidgets
      (bind _returnvalue (UserInterface|CreateWidget "/Game/Mods/LitManTestMod/LitMan_W_Physique.LitMan_W_Physique_C" (Game|GetPlayerController 0)))
      (Variables|Default|SetLitManWidget _returnvalue)
      (CallFunction|AddWidget _array_element))))

(event Custom|AddWidget
  (params (parent :type W%20Character%20Creation%20Main%20Object%20Reference))
  (Widget|Panel|AddChild (Variables|/Game/UI/CharacterCreation/W_CharacterCreation_Main.W_CharacterCreation_Main_C|GetMainPanel_Buttons parent) (Variables|Default|GetLitManWidget)))

(event EventBeginPlay)

(event EventTick
  (params (DeltaSeconds :type Float%20%28single-precision%29)))

(fn ConstructionScript)

(fn ModDataTableOperations
  (Class|ModController|MergeDataTables "/Game/Systems/SpawnTable/SpawnDataTable.SpawnDataTable" "/Game/Mods/LitManTestMod/Misc/SpawnDataTable.SpawnDataTable")
  (Class|ModController|MergeDataTables "/Game/Mods/LitManTestMod/Misc/EquipmentTemplateDataTable.EquipmentTemplateDataTable" "/Game/Systems/SpawnTable/EquipmentTemplateDataTable.EquipmentTemplateDataTable"))
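; Actor component for the LitManIncreasedWeight mod that massively raises the player's carry weight limit.
; One second after BeginPlay it casts its owner to BasePlayerChar and overwrites the base encumbrance in that character's encumbrance system with a huge fixed value.
; Unconnected leftover nodes would restore the base to a normal value or print it for debugging, but they never run.
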(event EventBeginPlay
  (Utilities|FlowControl|Delay 1.0)
  (bind _asbase_player_char (Utilities|Casting|CastToBasePlayerChar (Components|GetOwner)))
  (bind _output_get (Variables|/Game/Systems/Combat/EncumbranceSystem/BP_EncumbranceSystem.BP_EncumbranceSystem_C|SetEncumbranceBase (Variables|/Game/Characters/BasePlayerChar.BasePlayerChar_C|GetBP_EncumbranceSystem _asbase_player_char) 7e+06)))

(event EventTick
  (params (DeltaSeconds :type Float%20%28single-precision%29)))